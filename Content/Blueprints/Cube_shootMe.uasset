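; Target cube actor that counts how many times it is shot and shows the tally on a spinning text label.
; BeginPlay runs an endless short-Delay loop that yaws the TextRender one degree per step, wrapping back to zero at 360.
; The Shot event increments Hits and rewrites the label with a formatted shot count.
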(event `self.ReceiveBeginPlay`
  (bind _textrender (`self.TextRender`))
  (bind (_relativerotation_roll _relativerotation_pitch _relativerotation_yaw) (`KismetMathLibrary.BreakRotator` (`SceneComponent.RelativeRotation` _textrender)))
  (bind _returnvalue (+ _relativerotation_yaw 1.0))
  (if (< _returnvalue 360.0) :!label _label
    (`SceneComponent.K2_SetRelativeRotation` _textrender (`KismetMathLibrary.MakeRotator` _relativerotation_roll _relativerotation_pitch _returnvalue) false false)
    (else
      (`SceneComponent.K2_SetRelativeRotation` _textrender (`KismetMathLibrary.MakeRotator` _relativerotation_roll _relativerotation_pitch) false false)))
  (`KismetSystemLibrary.Delay` 0.005)
  (goto _label))

(event `Shot`
  (set `self.hits` (+ (`self.hits`) 1.0))
  (`TextRenderComponent.K2_SetText` (`self.TextRender`) (`|FormatText` "I've been shot {shots} times" (`self.hits`))))

(fn `UserConstructionScript`)