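; Ammo pickup actor that grants the first-person player five rounds when walked into.
; Box overlap casts to FirstPersonCharacter, adds to its Ammo, pushes the new count to its Ammotracker and calls Update, then destroys the pickup.
; From BeginPlay, a self-looping short Delay continuously spins the TextRender label in yaw, wrapping at a full turn, instead of using Tick.
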(event `self.ReceiveBeginPlay`
  (bind _textrender (`self.TextRender`))
  (bind (_relativerotation_roll _relativerotation_pitch _relativerotation_yaw) (`KismetMathLibrary.BreakRotator` (`SceneComponent.RelativeRotation` _textrender)))
  (bind _returnvalue (+ _relativerotation_yaw 1.0))
  (if (< _returnvalue 360.0) :!label _label
    (`SceneComponent.K2_SetRelativeRotation` _textrender (`KismetMathLibrary.MakeRotator` _relativerotation_roll _relativerotation_pitch _returnvalue) false false)
    (else
      (`SceneComponent.K2_SetRelativeRotation` _textrender (`KismetMathLibrary.MakeRotator` _relativerotation_roll _relativerotation_pitch) false false)))
  (`KismetSystemLibrary.Delay` 0.005)
  (goto _label))

(event `self.Box.OnComponentBeginOverlap`
  (params (OverlappedComponent :type "PrimitiveComponent Object Reference") (OtherActor :type "Actor Object Reference") (OtherComp :type "PrimitiveComponent Object Reference") (OtherBodyIndex :type Integer) (bFromSweep :type Boolean) (SweepResult :type "HitResult Structure (by ref)"))
  (bind _asfirst_person_character (cast `/Game/Blueprints/FirstPersonCharacter` OtherActor))
  (bind _output_get (set `/Game/Blueprints/FirstPersonCharacter.Ammo` (+ (`/Game/Blueprints/FirstPersonCharacter.Ammo` _asfirst_person_character) 5) _asfirst_person_character))
  (bind _ammotracker (`/Game/Blueprints/FirstPersonCharacter.ammotracker` _asfirst_person_character))
  (set `/Game/Widgets/AmmoTracker.Ammo` _output_get _ammotracker)
  (`/Game/Widgets/AmmoTracker.Update` _ammotracker)
  (`self.K2_DestroyActor`))

(fn `UserConstructionScript`)