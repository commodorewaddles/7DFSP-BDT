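; Cube_ouch is a damage-zone actor that hurts the FirstPersonCharacter while it overlaps the Box and displays that character's health.
; BeginPlay runs an endless short-Delay loop that spins the TextRender around yaw, wrapping at a full turn.
; Box overlap events toggle an Ouch flag, and Tick uses it to apply small per-frame damage to the overlapping character and update the text with its Health.
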(event `self.ReceiveBeginPlay`
  (bind _textrender (`self.TextRender`))
  (bind (_relativerotation_roll _relativerotation_pitch _relativerotation_yaw) (`KismetMathLibrary.BreakRotator` (`SceneComponent.RelativeRotation` _textrender)))
  (bind _returnvalue (+ _relativerotation_yaw 1.0))
  (if (< _returnvalue 360.0) :!label _label
    (`SceneComponent.K2_SetRelativeRotation` _textrender (`KismetMathLibrary.MakeRotator` _relativerotation_roll _relativerotation_pitch _returnvalue) false false)
    (else
      (`SceneComponent.K2_SetRelativeRotation` _textrender (`KismetMathLibrary.MakeRotator` _relativerotation_roll _relativerotation_pitch) false false)))
  (`KismetSystemLibrary.Delay` 0.005)
  (goto _label))

(event `self.Box.OnComponentBeginOverlap`
  (params (OverlappedComponent :type "PrimitiveComponent Object Reference") (OtherActor :type "Actor Object Reference") (OtherComp :type "PrimitiveComponent Object Reference") (OtherBodyIndex :type Integer) (bFromSweep :type Boolean) (SweepResult :type "HitResult Structure (by ref)"))
  (set `self.ouch?` true))

(event `self.Box.OnComponentEndOverlap`
  (params (OverlappedComponent :type "PrimitiveComponent Object Reference") (OtherActor :type "Actor Object Reference") (OtherComp :type "PrimitiveComponent Object Reference") (OtherBodyIndex :type Integer))
  (set `self.ouch?` false))

(event `self.ReceiveTick`
  (params (DeltaSeconds :type "Float (single-precision)"))
  (if (`self.ouch?`)
    (bind _asfirst_person_character (cast `/Game/Blueprints/FirstPersonCharacter` (stale `self.Box.OnComponentBeginOverlap` OtherActor)))
    (`/Game/Blueprints/FirstPersonCharacter.Take damage` _asfirst_person_character 0.01)
    (`TextRenderComponent.K2_SetText` (`self.TextRender`) (`KismetSystemLibrary.MakeLiteralText` (`KismetTextLibrary.Conv_DoubleToText` (`/Game/Blueprints/FirstPersonCharacter.Health` _asfirst_person_character) "HalfToEven")))))

(fn `UserConstructionScript`)