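; Game instance that manages a single-slot save game for the first-person player.
; On Init it loads the existing Save_file from the slot or creates a new one.
; SaveGame records the level name and character transform, then writes the slot, while ClearGame deletes it.
; LoadGame opens the saved level and immediately teleports the current character, without waiting for the level to load.
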(event `self.ReceiveInit`
  (bind _returnvalue (`GameplayStatics.DoesSaveGameExist` (`self.SlotName`)))
  (if _returnvalue
    (bind _returnvalue_2 (`GameplayStatics.LoadGameFromSlot` (`self.SlotName`)))
    (bind _assave_file (cast `/Game/Blueprints/Save_file` _returnvalue_2))
    (set `self.saveFile` _assave_file)
    (else
      (bind _returnvalue_3 (`GameplayStatics.CreateSaveGameObject` "/Game/Blueprints/Save_file.Save_file_C"))
      (set `self.saveFile` _returnvalue_3))))

(event `SaveGame`
  (bind _asfirst_person_character (cast `/Game/Blueprints/FirstPersonCharacter` (`GameplayStatics.GetPlayerCharacter` 0)))
  ;[1 1 1] Set save game to match each variable we care about
  (bind _returnvalue (`GameplayStatics.GetCurrentLevelName` true))
  (set `self.Current level` _returnvalue)
  (set `self.transform` (`Actor.GetTransform` _asfirst_person_character))
  (`GameplayStatics.SaveGameToSlot` (`self.saveFile`) (`self.SlotName`)))

(event `LoadGame`
  (bind _asfirst_person_character (cast `/Game/Blueprints/FirstPersonCharacter` (`GameplayStatics.GetPlayerCharacter` 0)))
  ;[1 1 1] Load the above variables
  (`GameplayStatics.OpenLevel` (`KismetStringLibrary.Conv_StringToName` (`self.Current level`)))
  (`Actor.K2_SetActorTransform` _asfirst_person_character (`self.transform`) false true))

(event `ClearGame`
  (`GameplayStatics.DeleteGameInSlot` (`self.SlotName`)))